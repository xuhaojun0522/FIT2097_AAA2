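; BinaryCombo is a three-digit combination lock actor that takes keyboard input from BeginPlay, with no proximity check.
; Keys 1/2/3 raise and Z/X/C lower each digit's text; increments wrap from 9 to 0, while decrements stop at 0.
; Each change compares the concatenated digits against Combo, turning the point light green on a match or red otherwise.
; A match also sets ComboCheck on the player character, which is never cleared here.
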(event EventBeginPlay
  (Utilities|Casting|CastToFIT2097_AAA2Character (Game|GetPlayerCharacter 0))
  (Input|EnableInput (Game|GetPlayerController 0)))

(event Collision|EventActorBeginOverlap
  (params (OtherActor :type Actor%20Object%20Reference)))

(event EventTick
  (params (DeltaSeconds :type Float%20%28single-precision%29)))

(event Input|KeyboardEvents|1
  (params (Key :type Key%20Structure))
  (:Released
    (CallFunction|Increment (Variables|Default|GetCode_1_up))
    (Utilities|Casting|CastToFIT2097_AAA2Character (Game|GetPlayerCharacter 0))))

(event Input|KeyboardEvents|Z
  (params (Key :type Key%20Structure))
  (:Released
    (CallFunction|Decrement (Variables|Default|GetCode_1_down))))

(event Input|KeyboardEvents|2
  (params (Key :type Key%20Structure))
  (:Released
    (CallFunction|Increment (Variables|Default|GetCode_2_up))))

(event Input|KeyboardEvents|X
  (params (Key :type Key%20Structure))
  (:Released
    (CallFunction|Decrement (Variables|Default|GetCode_2_down))))

(event Input|KeyboardEvents|C
  (params (Key :type Key%20Structure))
  (:Released
    (CallFunction|Decrement (Variables|Default|GetCode_3_down))))

(event Input|KeyboardEvents|3
  (params (Key :type Key%20Structure))
  (:Released
    (CallFunction|Increment (Variables|Default|GetCode_3_up))))

(fn ConstructionScript)

(fn Increment
  (params (CodeInput :type Static%20Mesh%20Component%20Object%20Reference))
  (Utilities|FlowControl|Sequence
    (:then_0
      (if (== CodeInput (Variables|Default|GetCode_1_up))
        (if (< (Variables|Default|GetCode_1_Value) 9)
          (Math|Integer|IncrementInt (Variables|Default|GetCode_1_Value)
            (:%20%20
              _))
          (else
            (Variables|Default|SetCode_1_Value 0)))
        (Rendering|Components|TextRender|SetText (Variables|Default|GetCode_1) (Utilities|Text|ToText(Integer) (Variables|Default|GetCode_1_Value)))
        (bind _actionon (CallFunction|ComboCheck :!label _label))
        (Utilities|Casting|CastToFIT2097_AAA2Character (Game|GetPlayerCharacter 0))
        (CallFunction|Action _actionon)))
    (:then_1
      (if (== CodeInput (Variables|Default|GetCode_2_up))
        (if (< (Variables|Default|GetCode_2_Value) 9)
          (Math|Integer|IncrementInt (Variables|Default|GetCode_2_Value)
            (:%20%20
              _))
          (else
            (Variables|Default|SetCode_2_Value 0)))
        (Rendering|Components|TextRender|SetText (Variables|Default|GetCode_2) (Utilities|Text|ToText(Integer) (Variables|Default|GetCode_2_Value)))
        (goto _label)))
    (:then_2
      (if (== CodeInput (Variables|Default|GetCode_3_up))
        (if (< (Variables|Default|GetCode_3_Value) 9)
          (Math|Integer|IncrementInt (Variables|Default|GetCode_3_Value)
            (:%20%20
              _))
          (else
            (Variables|Default|SetCode_3_Value 0)))
        (Rendering|Components|TextRender|SetText (Variables|Default|GetCode_3) (Utilities|Text|ToText(Integer) (Variables|Default|GetCode_3_Value)))
        (goto _label)))))

(fn ComboCheck
  (return (Utilities|Enum|Equal(Enum) (Variables|Default|GetCombo) (Utilities|String|Append (Utilities|String|ToString(Integer) (Variables|Default|GetCode_1_Value)) (Utilities|String|ToString(Integer) (Variables|Default|GetCode_2_Value)) (Utilities|String|ToString(Integer) (Variables|Default|GetCode_3_Value))))))

(fn Decrement
  (params (CodeInput :type Static%20Mesh%20Component%20Object%20Reference))
  (Utilities|FlowControl|Sequence
    (:then_0
      (if (== CodeInput (Variables|Default|GetCode_1_down))
        (if (> (Variables|Default|GetCode_1_Value) 0)
          (Math|Integer|DecrementInt (Variables|Default|GetCode_1_Value)
            (:%20%20
              _))
          (else
            (Variables|Default|SetCode_1_Value 0)))
        (Rendering|Components|TextRender|SetText (Variables|Default|GetCode_1) (Utilities|Text|ToText(Integer) (Variables|Default|GetCode_1_Value)))
        (bind _actionon (CallFunction|ComboCheck :!label _label))
        (Utilities|Casting|CastToFIT2097_AAA2Character (Game|GetPlayerCharacter 0))
        (CallFunction|Action _actionon)))
    (:then_1
      (if (== CodeInput (Variables|Default|GetCode_2_down))
        (if (> (Variables|Default|GetCode_2_Value) 0)
          (Math|Integer|DecrementInt (Variables|Default|GetCode_2_Value)
            (:%20%20
              _))
          (else
            (Variables|Default|SetCode_2_Value 0)))
        (Rendering|Components|TextRender|SetText (Variables|Default|GetCode_2) (Utilities|Text|ToText(Integer) (Variables|Default|GetCode_2_Value)))
        (goto _label)))
    (:then_2
      (if (== CodeInput (Variables|Default|GetCode_3_down))
        (if (> (Variables|Default|GetCode_3_Value) 0)
          (Math|Integer|DecrementInt (Variables|Default|GetCode_3_Value)
            (:%20%20
              _))
          (else
            (Variables|Default|SetCode_3_Value 0)))
        (Rendering|Components|TextRender|SetText (Variables|Default|GetCode_3) (Utilities|Text|ToText(Integer) (Variables|Default|GetCode_3_Value)))
        (goto _label)))))

(fn Action
  (params (Action%20On :type Boolean))
  (bind _pointlight (Variables|Default|GetPointLight))
  (if Action%20On
    (Rendering|Components|Light|SetLightColor _pointlight "(R=0.000000,G=1.000000,B=0.000000,A=1.000000)" true)
    (bind _asfit2097_aaa2character (Utilities|Casting|CastToFIT2097_AAA2Character (Game|GetPlayerCharacter 0)))
    (Variables|/Script/FIT2097_AAA2.FIT2097_AAA2Character|SetcomboCheck _asfit2097_aaa2character true)
    (else
      (Rendering|Components|Light|SetLightColor _pointlight "(R=1.000000,G=0.000000,B=0.000000,A=1.000000)" true))))