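; PoisonGas is a hazard Blueprint that steadily drains the player character's health, regardless of position, as its overlap event is empty.
; Tick runs a Delay that throttles damage to every few seconds, then lowers Health and HealthPercentage by fixed steps and prints the result.
; Once health is depleted, it pauses the game and creates the Die_Screen widget, with no Add to Viewport call here.
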(event EventBeginPlay)

(event Collision|EventActorBeginOverlap
  (params (OtherActor :type Actor%20Object%20Reference)))

(event EventTick
  (params (DeltaSeconds :type Float%20%28single-precision%29))
  (bind _asfit2097_aaa2character (Utilities|Casting|CastToFIT2097_AAA2Character (Game|GetPlayerCharacter 0)))
  (if (> (Variables|/Script/FIT2097_AAA2.FIT2097_AAA2Character|GetHealth _asfit2097_aaa2character) 0.0)
    (bind _asfit2097_aaa2character_2 (Utilities|Casting|CastToFIT2097_AAA2Character (Game|GetPlayerCharacter 0)))
    (Utilities|FlowControl|Delay 3.0)
    (bind _output_get (Variables|/Script/FIT2097_AAA2.FIT2097_AAA2Character|SetHealth _asfit2097_aaa2character_2 (- (Variables|/Script/FIT2097_AAA2.FIT2097_AAA2Character|GetHealth _asfit2097_aaa2character_2) 1e+01)))
    (Variables|/Script/FIT2097_AAA2.FIT2097_AAA2Character|SetHealthPercentage _asfit2097_aaa2character_2 (- (Variables|/Script/FIT2097_AAA2.FIT2097_AAA2Character|GetHealthPercentage _asfit2097_aaa2character_2) 0.1))
    (Development|PrintString (Utilities|String|ToString(Float) _output_get))
    (else
      (Game|SetGamePaused true)
      (UserInterface|CreateWidget "/Game/Blueprint/HUD_Widget/Die_Screen.Die_Screen_C"))))

(fn ConstructionScript)